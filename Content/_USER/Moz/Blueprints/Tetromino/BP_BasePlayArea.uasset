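; Base actor for a networked tetromino puzzle area that spawns falling blocks and scores surviving row entities (penguins).
; Server-to-client events spawn tetrominoes at the attach point, while CheckLines adds entities beside overlapping blocks.
; A block reaching EndTrigger nudges entities upward and polls until none remain, while arriving entities raise a RepNotify score sent to controllers.
; It then shows feedback and later returns the player to their saved transform in third person.
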(event `InitialStart`)

(event `FireStart`
  (bind _returnvalue (`GameplayStatics.GetGameMode`))
  (bind _attachpoint (`self.AttachPoint`))
  ;[1 1 1] Ask server to spawn tetromino
  (`KismetSystemLibrary.Delay` 5.0)
  (`self.Server_SpawnBase` :`Spawn Transform Location` (`SceneComponent.K2_GetComponentLocation` _attachpoint) :`Spawn Transform Rotation` (`SceneComponent.K2_GetComponentRotation` _attachpoint) :`U_CurrentBasePlayArea` self :`CurrentTetrominoRef` (`self.CreatedTetromino`))
  (bind _asbp_blockrun_gm (cast `/Game/_USER/Moz/Blueprints/BP_BlockrunGM` _returnvalue)
    (:`then`
      (`/Game/_USER/Moz/Blueprints/BP_BlockrunGM.SetCurrentPlayArea` _asbp_blockrun_gm self))
    (:`CastFailed`
      (bind _asbp_first_person_gm (cast `/Game/_USER/Moz/Blueprints/BP_FirstPersonGM` _returnvalue))
      (`/Game/_USER/Moz/Blueprints/BP_FirstPersonGM.SetCurrentPlayArea` _asbp_first_person_gm self))))

(event `self.ReceiveBeginPlay`
  (if (`self.StartPuzzle`)
    (`self.FireStart`)))

(event `Server_SpawnBase`
  (params (`Spawn Transform Location` :type "Vector Structure") (`Spawn Transform Rotation` :type "Rotator Structure") (U_CurrentBasePlayArea :type "/Game/_USER/Moz/Blueprints/Tetromino/BP_BasePlayArea Object Reference") (U_ShouldLoop :type Boolean) (U_AllBasePlayAreas :type "Array of /Game/_USER/Moz/Blueprints/Tetromino/BP_BasePlayArea Object Reference (by ref)") (CurrentTetrominoRef :type "/Game/_USER/Moz/Blueprints/Tetromino/BP_BaseBlock Object Reference"))
  (bind _attachpoint (`self.AttachPoint`))
  (`self.Client_SpawnBaseOnClient` (`SceneComponent.K2_GetComponentLocation` _attachpoint) (`SceneComponent.K2_GetComponentRotation` _attachpoint) U_CurrentBasePlayArea U_ShouldLoop U_AllBasePlayAreas CurrentTetrominoRef))

(event `Client_SpawnBaseOnClient`
  (params (`Spawn Transform Location` :type "Vector Structure") (`Spawn Transform Rotation` :type "Rotator Structure") (U_CurrentBasePlayArea :type "/Game/_USER/Moz/Blueprints/Tetromino/BP_BasePlayArea Object Reference") (U_ShouldLoop :type Boolean) (U_AllBasePlayAreas :type "Array of /Game/_USER/Moz/Blueprints/Tetromino/BP_BasePlayArea Object Reference (by ref)") (CurrentTetrominoRef :type "/Game/_USER/Moz/Blueprints/Tetromino/BP_BaseBlock Object Reference"))
  (bind _createdtetromino (`self.StartSpawner` `Spawn Transform Location` `Spawn Transform Rotation` U_CurrentBasePlayArea U_ShouldLoop U_AllBasePlayAreas CurrentTetrominoRef))
  (bind _asbp_blockrun_gm (cast `/Game/_USER/Moz/Blueprints/BP_BlockrunGM` (`GameplayStatics.GetGameMode`)))
  (`/Game/_USER/Moz/Blueprints/BP_BlockrunGM.SetCurrentTetromino` _asbp_blockrun_gm _createdtetromino))

(event `self.EndTrigger.OnComponentBeginOverlap`
  (params (OverlappedComponent :type "PrimitiveComponent Object Reference") (OtherActor :type "Actor Object Reference") (OtherComp :type "PrimitiveComponent Object Reference") (OtherBodyIndex :type Integer) (bFromSweep :type Boolean) (SweepResult :type "HitResult Structure (by ref)"))
  (bind _rowfullentities (`self.RowFullEntities`))
  (bind (_returnvalue_x _returnvalue_y _returnvalue_z) (`KismetMathLibrary.BreakVector` (`SceneComponent.K2_GetComponentLocation` (`self.EndTrigger`))))
  ;[1 1 1] On hitting the end zone, step by step advance entities; then check for the array with all entities and continue doing the move up (Reach Target Z) until atleast 1 entity remains
  (cast `/Game/_USER/Moz/Blueprints/Tetromino/BP_BaseSingleBlock` OtherActor
    (:`then`
      (`KismetSystemLibrary.PrintString` "END")
      (bind _returnvalue (`KismetSystemLibrary.K2_SetTimerDelegate` (delegate `CheckForLevelEnd`) 1.0 true))
      (set `self.U_HasReachedEnd` true)
      (if (not (`KismetArrayLibrary.Array_IsEmpty` _rowfullentities))
        (for _array_element _rowfullentities :!label _label
          (`/Engine/EditorBlueprintResources/StandardMacros.IsValid` _array_element
            (:`Is Valid`
              (bind _asbp_row_spawned_entity (cast `/Game/_USER/Moz/Blueprints/Objects/BP_RowSpawnedEntity` _array_element))
              (bind (_returnvalue_x_2 _returnvalue_y_2 _returnvalue_z_2) (`KismetMathLibrary.BreakVector` (`self.K2_GetActorLocation` _asbp_row_spawned_entity)))
              (if (not (== _returnvalue_z_2 _returnvalue_z))
                (set `/Game/_USER/Moz/Blueprints/Objects/BP_RowSpawnedEntity.TargetZ` (+ _returnvalue_z_2 (`KismetMathLibrary.RandomFloatInRange` 20.0 50.0)) _asbp_row_spawned_entity)
                (`|ExecutionSequence`
                  (:`then_0`
                    (`KismetSystemLibrary.Delay` 0.5)
                    (goto _label)))))
            (:`Is Not Valid`
              (`KismetArrayLibrary.Array_RemoveItem` _rowfullentities _array_element)
              (goto _label))))))
    (:`CastFailed`
      (bind _asbp_row_spawned_entity_2 (cast `/Game/_USER/Moz/Blueprints/Objects/BP_RowSpawnedEntity` OtherActor))
      (`/Engine/EditorBlueprintResources/StandardMacros.IsValid` _asbp_row_spawned_entity_2
        (:`Is Valid`
          (`self.IncreaseScore` _asbp_row_spawned_entity_2))))))

(event `CheckForLevelEnd`
  (bind _currentplayerinlevel (`self.CurrentPlayerInLevel`))
  ;[1 1 1] On hitting the end zone, step by step advance entities; then check for the array with all entities and continue doing the move up (Reach Target Z) until atleast 1 entity remains
  (if (and (`KismetArrayLibrary.Array_IsEmpty` (`self.RowFullEntities`)) (`self.U_HasReachedEnd`))
    (set `self.OverallEnd` true)
    (else
      (set `self.OverallEnd` false)))
  (if (`self.OverallEnd`)
    (`KismetSystemLibrary.K2_ClearAndInvalidateTimerHandle` (stale `self.EndTrigger.OnComponentBeginOverlap` _returnvalue))
    (`/Engine/EditorBlueprintResources/StandardMacros.IsValid` _currentplayerinlevel
      (:`Is Valid`
        (`/Game/_USER/Moz/Blueprints/BP_BlockrunController.Server_DisplayFeedback` _currentplayerinlevel self true))
      (:`Is Not Valid`
        (bind _asbp_first_person_gm (cast `/Game/_USER/Moz/Blueprints/BP_FirstPersonGM` (`GameplayStatics.GetGameMode`))
          (:`then`
            (bind _asbp_blockrun_controller (cast `/Game/_USER/Moz/Blueprints/BP_BlockrunController` (`/Game/_USER/Moz/Blueprints/BP_FirstPersonGM.CurrentPuzzlePlayerOnServer` _asbp_first_person_gm)))
            (`KismetSystemLibrary.PrintString` (`KismetSystemLibrary.GetDisplayName` _asbp_blockrun_controller))
            (`/Game/_USER/Moz/Blueprints/BP_BlockrunController.Server_DisplayFeedback` _asbp_blockrun_controller self false))
          (:`CastFailed`
            (`KismetSystemLibrary.PrintString` "cast to fpgm failed")))))))

(event `IncreaseScore`
  (params (InEntityObject :type "Object Object Reference"))
  ;[1 1 1] When hitting the last checkzone (before end zone) add to the score
  (if (== (`GameplayStatics.GetObjectClass` InEntityObject) "/Game/_USER/Moz/Blueprints/Objects/BP_RowSpawnedEntity.BP_RowSpawnedEntity_C")
    (bind _output_get (set `self.SurvivingEntities` (+ (`self.SurvivingEntities`) 1)))
    (`KismetSystemLibrary.PrintString` (`KismetStringLibrary.Conv_IntToString` _output_get))))

(event `MoveEntities`
  ;[1 0 0] Move entities one block after its spawned (OBSOLETE)
)

(event `DetectInLoadingZone`
  (params (InputObject :type "Object Object Reference"))
  ;[1 1 1] Once player enters loading zone, save the value of where to return (in this door bp) to the player so that they "remember"
  (`/Engine/EditorBlueprintResources/StandardMacros.IsValid` InputObject
    (:`Is Valid`
      (bind _asbp_blockrun_controller (cast `/Game/_USER/Moz/Blueprints/BP_BlockrunController` InputObject))
      (bind _output_get (set `self.CurrentPlayerInLevel` _asbp_blockrun_controller))
      (set `self.TeleportOutTransform` (`/Game/_USER/Moz/Blueprints/BP_BlockrunController.ReturnZoneLoc` _output_get))
      (`KismetSystemLibrary.PrintString` "Got return zone from player"))
    (:`Is Not Valid`
      (bind _asbp_blockrun_char_f (cast `/Game/_USER/Moz/Blueprints/Character/BP_BlockrunCharF` InputObject)
        (:`then`
          (bind _asbp_blockrun_controller_2 (cast `/Game/_USER/Moz/Blueprints/BP_BlockrunController` (`Pawn.GetController` _asbp_blockrun_char_f)))
          (bind _output_get_2 (set `self.CurrentPlayerInLevel` _asbp_blockrun_controller_2)))
        (:`CastFailed`
          (`KismetSystemLibrary.PrintString` (`KismetSystemLibrary.GetDisplayName` _output_get_2) true true (struct :`R` 1.0 :`G` 0.143357 :`A` 1.0)))))))

(event `self.PlayerDetectionZone.OnComponentBeginOverlap`
  (params (OverlappedComponent :type "PrimitiveComponent Object Reference") (OtherActor :type "Actor Object Reference") (OtherComp :type "PrimitiveComponent Object Reference") (OtherBodyIndex :type Integer) (bFromSweep :type Boolean) (SweepResult :type "HitResult Structure (by ref)"))
  (`self.DetectInLoadingZone` (`self.GetInstigatorController` OtherActor)))

(event `PostFeedbackEnd`
  (bind _currentplayerinlevel (`self.CurrentPlayerInLevel`))
  ;[1 1 1] Once Feedback is over, spawn the player to the outside of the level (back to original level)
  (if (or (`self.FeedbackDone`) (`self.ExitScoreScreen`))
    (`WidgetBlueprintLibrary.SetInputMode_GameOnly` _currentplayerinlevel)
    (`Widget.RemoveFromParent` (`/Game/_USER/Moz/Blueprints/BP_BlockrunController.CurrentScoreScreen` _currentplayerinlevel))
    (set `PlayerController.bShowMouseCursor` false _currentplayerinlevel)
    (`/Game/_USER/Moz/Blueprints/BP_BlockrunController.Server_SetSpawnTransform` _currentplayerinlevel (`self.TeleportOutTransform`))
    (`/Game/_USER/Moz/Blueprints/BP_BlockrunController.Server_SpawnToLocation` _currentplayerinlevel false)
    (bind _asbp_blockrun_char_f (cast `/Game/_USER/Moz/Blueprints/Character/BP_BlockrunCharF` (`Controller.K2_GetPawn` _currentplayerinlevel)))
    (`/Game/_USER/Moz/Blueprints/Character/BP_BlockrunCharF.SwitchToThirdPerson` _asbp_blockrun_char_f)
    (set `self.FeedbackDone` false)))

(event `PostScoreScreenEnd`
  ;[1 0 0] Technically not needed
  (if (`self.ExitScoreScreen`)
    _))

(event `PostScoreScreenRestart`
  ;[1 0 0] Technically not needed
  (if (`self.ExitScoreScreen`)
    _))

(fn `CheckLines`
  (returns (EntitiesSpawned :type Boolean))
  (locals (localOverlappingActors :type "Array of Actor Object Reference") (localDropAmount :type "Float (double-precision)") (localCutoffLineZ :type "Float (double-precision)" :default 2000.0) (localDropAmountNeg :type "Float (double-precision)" :default 2000.0))
  (bind _output_get (set `self.AllBoxColliders` (`self.K2_GetComponentsByClass` "/Script/Engine.BoxComponent")))
  ;[1 1 1] Once a row is complete, add entities (penguins) to that row for movement
  (for _array_element (`PrimitiveComponent.GetOverlappingActors` (`|GetArrayItem` _output_get) "/Game/_USER/Moz/Blueprints/Tetromino/BP_BaseSingleBlock.BP_BaseSingleBlock_C")
    (bind _asbp_base_single_block (cast `/Game/_USER/Moz/Blueprints/Tetromino/BP_BaseSingleBlock` _array_element))
    (`/Game/_USER/Moz/Blueprints/Tetromino/BP_BaseSingleBlock.AddEntitiesAfterRow` _asbp_base_single_block (`KismetMathLibrary.MakeTransform` (+ (`self.K2_GetActorLocation` _asbp_base_single_block) (0.0 50.0 0.0))))
    (`KismetArrayLibrary.Array_AddUnique` (`self.RowFullEntities`) (`/Game/_USER/Moz/Blueprints/Tetromino/BP_BaseSingleBlock.CurrentSingleSpawnedEntity` _asbp_base_single_block))
    (set `self.RowFullEntitiesSpawned` true)))

(fn `GetAttachTransform`
  (returns (AttachTransform :type "Transform Structure"))
  (return (`SceneComponent.K2_GetComponentToWorld` (`self.AttachPoint`))))

(fn `OnRep_CounterTillCamMovement`)

(fn `OnRep_SurvivingEntities`
  (bind _outactors (`GameplayStatics.GetAllActorsOfClass` "/Game/_USER/Moz/Blueprints/BP_BlockrunController.BP_BlockrunController_C"))
  (for _array_element _outactors
    (`/Game/_USER/Moz/Blueprints/BP_BlockrunController.Server_UpdateEntitySavedScore` _array_element (`self.SurvivingEntities`) _array_element)))

(fn `StartSpawner`
  (params (`Spawn Transform Location` :type "Vector Structure") (`Spawn Transform Rotation` :type "Rotator Structure") (U_CurrentBasePlayArea :type "/Game/_USER/Moz/Blueprints/Tetromino/BP_BasePlayArea Object Reference") (U_ShouldLoop :type Boolean) (U_AllBasePlayAreas :type "Array of /Game/_USER/Moz/Blueprints/Tetromino/BP_BasePlayArea Object Reference") (CurrentTetrominoRef :type "/Game/_USER/Moz/Blueprints/Tetromino/BP_BaseBlock Object Reference"))
  (returns (CreatedTetromino :type "/Game/_USER/Moz/Blueprints/Tetromino/BP_BaseBlock Object Reference"))
  (bind _returnvalue (`|SpawnActorFromClass` "/Game/_USER/Moz/Blueprints/Tetromino/BP_BaseBlock.BP_BaseBlock_C" (`KismetMathLibrary.MakeTransform` `Spawn Transform Location` `Spawn Transform Rotation`) "Undefined" "MultiplyWithRoot" null false U_CurrentBasePlayArea U_ShouldLoop U_AllBasePlayAreas CurrentTetrominoRef null "0.000000,0.000000,0.000000|0.000000,0.000000,-0.000000|1.000000,1.000000,1.000000" 0 null))
  (bind _output_get (set `self.CreatedTetromino` _returnvalue))
  (return _output_get))

(fn `UserConstructionScript`
  (locals (localInitialChecklineLocation :type "Vector Structure" :default (0.0 0.0 0.0))))