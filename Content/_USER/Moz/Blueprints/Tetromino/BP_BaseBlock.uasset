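; Falling Tetris piece that shapes and colors four cubes into one of seven tetrominoes, chosen from BP_BlockrunGM's list or randomly.
; Input applies moves and rotations, reverting on box overlap; only moves replicate via server RPC and multicast.
; A looping timer drops it until downward traces hit.
; On landing, it spawns single blocks, has the play area check lines and spawn the next piece, then destroys itself.
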(event `EnhancedInput|/Game/_USER/Moz/Blueprints/Input/Tetris/IA_TurnCCLK`
  (params (ActionValue :type Boolean) (ElapsedSeconds :type "Float (double-precision)") (TriggeredSeconds :type "Float (double-precision)") (InputAction :type "InputAction Object Reference" :default "/Game/_USER/Moz/Blueprints/Input/Tetris/IA_TurnCCLK.IA_TurnCCLK"))
  ;[1 1 1] Turn Clockwise Custom Code - had to do it this way because without it the tetros freak out on inputs
  (:`Started`
    (`self.K2_AddActorLocalRotation` (struct :`Roll` 90.0))
    (for _array_element (`self.K2_GetComponentsByClass` "/Script/Engine.StaticMeshComponent")
      (bind (_outactors _returnvalue) (`KismetSystemLibrary.BoxOverlapActors` (`SceneComponent.K2_GetComponentLocation` _array_element) (15.0 15.0 15.0) (`|MakeArray` "ObjectTypeQuery1" :!type "EObjectTypeQuery Enum")))
      (if _returnvalue
        (`self.K2_AddActorLocalRotation` (struct :`Roll` -90.0))
        (break)))))

(event `EnhancedInput|/Game/_USER/Moz/Blueprints/Input/Tetris/IA_MoveBlockLeft`
  (params (ActionValue :type Boolean) (ElapsedSeconds :type "Float (double-precision)") (TriggeredSeconds :type "Float (double-precision)") (InputAction :type "InputAction Object Reference" :default "/Game/_USER/Moz/Blueprints/Input/Tetris/IA_MoveBlockLeft.IA_MoveBlockLeft"))
  (:`Started`
    (bind _newlocation (`self.Try Lateral Movement` -50.0))
    (`self.Server_UpdatePos` self (.location _newlocation) (.rotation _newlocation))))

(event `EnhancedInput|/Game/_USER/Moz/Blueprints/Input/Tetris/IA_TurnCLK`
  (params (ActionValue :type Boolean) (ElapsedSeconds :type "Float (double-precision)") (TriggeredSeconds :type "Float (double-precision)") (InputAction :type "InputAction Object Reference" :default "/Game/_USER/Moz/Blueprints/Input/Tetris/IA_TurnCLK.IA_TurnCLK"))
  (:`Started`
    (`self.K2_AddActorLocalRotation` (struct :`Roll` -90.0))
    (for _array_element (`self.K2_GetComponentsByClass` "/Script/Engine.StaticMeshComponent")
      (bind (_outactors _returnvalue) (`KismetSystemLibrary.BoxOverlapActors` (`SceneComponent.K2_GetComponentLocation` _array_element) (15.0 15.0 15.0) (`|MakeArray` "ObjectTypeQuery1" :!type "EObjectTypeQuery Enum")))
      (if _returnvalue
        (`self.K2_AddActorLocalRotation` (struct :`Roll` 90.0))
        (break)))))

(event `EnhancedInput|/Game/_USER/Moz/Blueprints/Input/Tetris/IA_MoveBlockRight`
  (params (ActionValue :type Boolean) (ElapsedSeconds :type "Float (double-precision)") (TriggeredSeconds :type "Float (double-precision)") (InputAction :type "InputAction Object Reference" :default "/Game/_USER/Moz/Blueprints/Input/Tetris/IA_MoveBlockRight.IA_MoveBlockRight"))
  (:`Started`
    (bind _newlocation (`self.Try Lateral Movement` 50.0))
    (`self.Server_UpdatePos` self (.location _newlocation) (.rotation _newlocation))))

(event `Server_UpdatePos`
  (params (`New Transform Location` :type "Vector Structure") (`New Transform Rotation` :type "Rotator Structure"))
  (`self.Multi_UpdatePos` self `New Transform Location` `New Transform Rotation`))

(event `Multi_UpdatePos`
  (params (`New Transform Location` :type "Vector Structure") (`New Transform Rotation` :type "Rotator Structure"))
  (`self.K2_SetActorTransform` self (`KismetMathLibrary.MakeTransform` `New Transform Location` `New Transform Rotation`) false false))

(event `EnhancedInput|/Game/_USER/Moz/Blueprints/Input/Tetris/IA_SpeedDescent`
  (params (ActionValue :type Boolean) (ElapsedSeconds :type "Float (double-precision)") (TriggeredSeconds :type "Float (double-precision)") (InputAction :type "InputAction Object Reference" :default "/Game/_USER/Moz/Blueprints/Input/Tetris/IA_SpeedDescent.IA_SpeedDescent"))
  (:`Triggered`
    (if ActionValue
      (if (not (`/Game/_USER/Moz/Blueprints/Tetromino/BP_BasePlayArea.U_HasReachedEnd` (stale `self.ReceiveBeginPlay` _output_get_3)))
        (bind _newlocation (`self.Try Lateral Movement` -50.0 true))
        (`self.Server_UpdatePos` self (.location _newlocation) (.rotation _newlocation))))))

(event `self.ReceiveBeginPlay`
  ;[1 1 1] Other Player is connected and is making Tetrominos
  (bind _asbp_blockrun_gm (cast `/Game/_USER/Moz/Blueprints/BP_BlockrunGM` (`GameplayStatics.GetGameMode`))
    (:`then`
      (bind _outfirstindex (`/Game/_USER/Moz/Blueprints/BP_BlockrunGM.ReturnFirstOfArray` _asbp_blockrun_gm (`/Game/_USER/Moz/Blueprints/BP_BlockrunGM.GeneratedTetroList` _asbp_blockrun_gm)))
      (`self.Server_CreateTetromino` _outfirstindex))
    (:`CastFailed`
      ;[1 1 1] Singleplayer mode, spawn random tetros
      (bind _output_get (set `self.RandomTetroID` (`KismetMathLibrary.RandomIntegerInRange` 0 6)))
      (`self.Server_CreateTetromino` _output_get)))
  (`self.Server_UpdateCurrentPC`)
  (`KismetSystemLibrary.PrintString` (`KismetSystemLibrary.GetDisplayName` (`self.CurrentOwnerPlayerController`)) true true (struct :`R` 0.911957 :`G` 1.0 :`A` 1.0))
  (bind _outactors (`GameplayStatics.GetAllActorsOfClass` "/Game/_USER/Moz/Blueprints/Tetromino/BP_BasePlayArea.BP_BasePlayArea_C"))
  (bind _output_get_2 (set `self.U_AllBasePlayAreas` _outactors))
  (bind _output (`|GetArrayItem` _output_get_2))
  (`/Engine/EditorBlueprintResources/StandardMacros.IsValid` _output
    (:`Is Valid`
      (bind _output_get_3 (set `self.U_CurrentBasePlayArea` _output))
      (if (`/Game/_USER/Moz/Blueprints/Tetromino/BP_BasePlayArea.U_HasReachedEnd` _output_get_3)
        (`self.K2_DestroyActor`)
        (`GameplayStatics.SetGlobalTimeDilation` 1.0)
        (else
          (bind _returnvalue (`KismetSystemLibrary.K2_SetTimerDelegate` (delegate `BlockDrop`) (`self.U_DropSpeed`) true))
          (set `self.U_BlockDroppingTimer` _returnvalue))))))

(event `BlockDrop`
  (bind _u_currentbaseplayarea (`self.U_CurrentBasePlayArea`))
  ;[1 1 1] Checking each Cube (x4) in the root component to see if any one is touching anything else
  (set `self.U_ShouldBlockDrop` true)
  (for _array_element (`SceneComponent.GetChildrenComponents` (`self.DefaultSceneRoot`) false)
    (bind _returnvalue (`SceneComponent.K2_GetComponentLocation` _array_element))
    ;;[1 1 1] Raycast downwards 50 units to see if anything else (static world elements) is present
    (bind (_outhit _returnvalue_2) (`KismetSystemLibrary.LineTraceSingleForObjects` _returnvalue (- _returnvalue (0.0 0.0 50.0)) (`|MakeArray` "ObjectTypeQuery1" :!type "EObjectTypeQuery Enum")))
    (if _returnvalue_2
      (`/Engine/EditorBlueprintResources/StandardMacros.DoOnce` false
        (:`Completed`
          (set `self.U_ShouldBlockDrop` false)
          (`KismetSystemLibrary.K2_ClearAndInvalidateTimerHandle` (`self.U_BlockDroppingTimer`))))))
  (if (`self.U_ShouldBlockDrop`)
    (`SceneComponent.K2_AddWorldOffset` (`self.DefaultSceneRoot`) (0.0 0.0 -50.0) false false)
    (else
      (for _array_element_2 (`SceneComponent.GetChildrenComponents` (`self.DefaultSceneRoot`) false)
        (`|SpawnActorFromClass` "/Game/_USER/Moz/Blueprints/Tetromino/BP_BaseSingleBlock.BP_BaseSingleBlock_C" (`KismetMathLibrary.MakeTransform` (`SceneComponent.K2_GetComponentLocation` _array_element_2)) "Undefined" "MultiplyWithRoot" null (`self.U_TetrominoColor`) null null))
      ;[1 1 1] Use this for how tetris destroys rows of blocks
      (`/Game/_USER/Moz/Blueprints/Tetromino/BP_BasePlayArea.CheckLines` _u_currentbaseplayarea)
      ;[1 1 1] Basically ShouldBlockDrop is false and the block has landed on base; change 1400 to whatever value is fit
      (`/Game/_USER/Moz/Blueprints/Tetromino/BP_BasePlayArea.Server_SpawnBase` _u_currentbaseplayarea (0.0 0.0 1100.0) (struct :`Yaw` -90.0) _u_currentbaseplayarea true (`self.U_AllBasePlayAreas`) (stale _output_get))
      (bind _output_get (set `/Game/_USER/Moz/Blueprints/Tetromino/BP_BasePlayArea.CreatedTetromino` (stale `Client_CreateTetromino` _output_get) _u_currentbaseplayarea))
      (`self.K2_DestroyActor`))))

(event `Client_UpdateCurrentPC`
  (bind _asbp_blockrun_gm (cast `/Game/_USER/Moz/Blueprints/BP_BlockrunGM` (`GameplayStatics.GetGameMode`)))
  (bind _asbp_blockrun_controller (cast `/Game/_USER/Moz/Blueprints/BP_BlockrunController` (`/Game/_USER/Moz/Blueprints/BP_BlockrunGM.CurrentPuzzlePlayerOnServer` _asbp_blockrun_gm)))
  (set `self.CurrentOwnerPlayerController` _asbp_blockrun_controller))

(event `Server_UpdateCurrentPC`
  (`self.Client_UpdateCurrentPC`))

(event `Server_CreateTetromino`
  (params (Selection :type Integer))
  ;[1 1 1] Call to server to create tetromino then server calls all clients to draw tetromino
  (`self.Client_CreateTetromino` Selection))

(event `Client_CreateTetromino`
  (params (Selection :type Integer))
  ;[1 1 1] Call to server to create tetromino then server calls all clients to draw tetromino
  ;;[1 0.6755 0] Change this back to Multicast if issues arise
  (bind _currenttetromino (`self.Create Tetromino` Selection))
  (bind _output_get (set `self.CurrentTetrominoRef` _currenttetromino))
  (`self.Server_SetTetrominoRef`))

(event `Client_SetTetrominoRef`
  ;[1 1 1] Call to server to store current tetromino block and then tell to clients
  ;;[1 0.7832 0] Change to Multi if issues
  (bind _asbp_blockrun_gm (cast `/Game/_USER/Moz/Blueprints/BP_BlockrunGM` (`GameplayStatics.GetGameMode`)))
  (`/Game/_USER/Moz/Blueprints/BP_BlockrunGM.SetCurrentTetromino` _asbp_blockrun_gm (`self.CurrentTetrominoRef`)))

(event `Server_SetTetrominoRef`
  ;[1 1 1] Call to server to store current tetromino block and then tell to clients
  (`self.Client_SetTetrominoRef`))

(event `Client_UpdateTetromino`)

(fn `Create Tetromino`
  (params (Selection :type Integer))
  (returns (CurrentTetromino :type "/Game/_USER/Moz/Blueprints/Tetromino/BP_BaseBlock Object Reference"))
  (switch `int` Selection
    (:`0`
      ;[1 1 1] Tetromino I
      (`SceneComponent.K2_AddLocalOffset` (`self.Cube2`) (0.0 0.0 50.0) false false)
      (`SceneComponent.K2_AddLocalOffset` (`self.Cube3`) (0.0 0.0 100.0) false false)
      (`SceneComponent.K2_AddLocalOffset` (`self.Cube4`) (0.0 0.0 150.0) false false)
      (set `self.U_TetrominoColor` (`|GetArrayItem` (`self.TetrominoColorArray`)))
      (set `self.U_CurrentTypeHeight` 300.0))
    (:`1`
      ;[1 1 1] Tetromino L
      (`SceneComponent.K2_AddLocalOffset` (`self.Cube2`) (0.0 0.0 50.0) false false)
      (`SceneComponent.K2_AddLocalOffset` (`self.Cube3`) (0.0 0.0 100.0) false false)
      (`SceneComponent.K2_AddLocalOffset` (`self.Cube4`) (0.0 50.0 0.0) false false)
      (set `self.U_TetrominoColor` (`|GetArrayItem` (`self.TetrominoColorArray`) 1))
      (set `self.U_CurrentTypeHeight` 150.0))
    (:`2`
      ;[1 1 1] Tetromino J
      (`SceneComponent.K2_AddLocalOffset` (`self.Cube2`) (0.0 0.0 50.0) false false)
      (`SceneComponent.K2_AddLocalOffset` (`self.Cube3`) (0.0 0.0 100.0) false false)
      (`SceneComponent.K2_AddLocalOffset` (`self.Cube4`) (0.0 -50.0 0.0) false false)
      (set `self.U_TetrominoColor` (`|GetArrayItem` (`self.TetrominoColorArray`) 2))
      (set `self.U_CurrentTypeHeight` 150.0))
    (:`3`
      ;[1 1 1] Tetromino O
      (`SceneComponent.K2_AddLocalOffset` (`self.Cube2`) (0.0 0.0 50.0) false false)
      (`SceneComponent.K2_AddLocalOffset` (`self.Cube3`) (0.0 50.0 0.0) false false)
      (`SceneComponent.K2_AddLocalOffset` (`self.Cube4`) (0.0 50.0 50.0) false false)
      (set `self.U_TetrominoColor` (`|GetArrayItem` (`self.TetrominoColorArray`) 3))
      (set `self.U_CurrentTypeHeight` 100.0))
    (:`4`
      ;[1 1 1] Tetromino S
      (`SceneComponent.K2_AddLocalOffset` (`self.Cube2`) (0.0 0.0 50.0) false false)
      (`SceneComponent.K2_AddLocalOffset` (`self.Cube3`) (0.0 50.0 50.0) false false)
      (`SceneComponent.K2_AddLocalOffset` (`self.Cube4`) (0.0 50.0 100.0) false false)
      (set `self.U_TetrominoColor` (`|GetArrayItem` (`self.TetrominoColorArray`) 4))
      (set `self.U_CurrentTypeHeight` 200.0))
    (:`5`
      ;[1 1 1] Tetromino T
      (`SceneComponent.K2_AddLocalOffset` (`self.Cube2`) (0.0 -50.0 0.0) false false)
      (`SceneComponent.K2_AddLocalOffset` (`self.Cube3`) (0.0 50.0 0.0) false false)
      (`SceneComponent.K2_AddLocalOffset` (`self.Cube4`) (0.0 0.0 50.0) false false)
      (set `self.U_TetrominoColor` (`|GetArrayItem` (`self.TetrominoColorArray`) 5))
      (set `self.U_CurrentTypeHeight` 50.0))
    (:`6`
      ;[1 1 1] Tetromino Z
      (`SceneComponent.K2_AddLocalOffset` (`self.Cube2`) (0.0 0.0 50.0) false false)
      (`SceneComponent.K2_AddLocalOffset` (`self.Cube3`) (0.0 -50.0 50.0) false false)
      (`SceneComponent.K2_AddLocalOffset` (`self.Cube4`) (0.0 -50.0 100.0) false false)
      (set `self.U_TetrominoColor` (`|GetArrayItem` (`self.TetrominoColorArray`) 6))
      (set `self.U_CurrentTypeHeight` 200.0)))
  (`MeshComponent.SetVectorParameterValueOnMaterials` (`self.Cube1`) "FloorColor" (`KismetMathLibrary.Conv_LinearColorToVector` (`self.U_TetrominoColor`)))
  (`MeshComponent.SetVectorParameterValueOnMaterials` (`self.Cube2`) "FloorColor" (`KismetMathLibrary.Conv_LinearColorToVector` (`self.U_TetrominoColor`)))
  (`MeshComponent.SetVectorParameterValueOnMaterials` (`self.Cube3`) "FloorColor" (`KismetMathLibrary.Conv_LinearColorToVector` (`self.U_TetrominoColor`)))
  (`MeshComponent.SetVectorParameterValueOnMaterials` (`self.Cube4`) "FloorColor" (`KismetMathLibrary.Conv_LinearColorToVector` (`self.U_TetrominoColor`)))
  (return self))

(fn `OnRep_CurrentTetrominoRef`)

(fn `OnRep_TurnCLK`)

(fn `Try Lateral Movement`
  (params (MoveAmount :type "Float (double-precision)") (DownMovement :type Boolean))
  (returns (NewLocation :type "Transform Structure"))
  (if DownMovement
    (`self.K2_AddActorWorldOffset` (`KismetMathLibrary.MakeVector` 0.0 0.0 MoveAmount))
    (for _array_element (`self.K2_GetComponentsByClass` "/Script/Engine.StaticMeshComponent")
      (bind (_outactors _returnvalue) (`KismetSystemLibrary.BoxOverlapActors` (`SceneComponent.K2_GetComponentLocation` _array_element) (15.0 15.0 15.0) (`|MakeArray` "ObjectTypeQuery1" :!type "EObjectTypeQuery Enum")))
      (if _returnvalue
        (`self.K2_AddActorWorldOffset` (`KismetMathLibrary.MakeVector` 0.0 0.0 (* MoveAmount -1.0)))
        (break)))
    (set `self.AfterLateralTransform` (`self.GetTransform`))
    (return (`self.AfterLateralTransform`))
    (else
      (`self.K2_AddActorWorldOffset` (`KismetMathLibrary.MakeVector` MoveAmount))
      (for _array_element_2 (`self.K2_GetComponentsByClass` "/Script/Engine.StaticMeshComponent")
        (bind (_outactors_2 _returnvalue_2) (`KismetSystemLibrary.BoxOverlapActors` (`SceneComponent.K2_GetComponentLocation` _array_element_2) (15.0 15.0 15.0) (`|MakeArray` "ObjectTypeQuery1" :!type "EObjectTypeQuery Enum")))
        (if _returnvalue_2
          (`self.K2_AddActorWorldOffset` (`KismetMathLibrary.MakeVector` (* MoveAmount -1.0)))
          (break)))
      (set `self.AfterLateralTransform` (`self.GetTransform`))
      (return (`self.AfterLateralTransform`)))))

(fn `UserConstructionScript`)