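; Carving puzzle actor that identifies which tetromino the player carved from the hit grid components.
; It splits component names into row and column letters, tallies them, and tests the counts against I, J, L, T, O, S and Z patterns; Z and T are noted as broken.
; The shape ID passes through server and client events to BP_BlockrunGM.
; On lock-in with a result, it respawns the player in third person, destroys itself and unloads the streamed level.
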(event `self.ReceiveTick`
  (params (DeltaSeconds :type "Float (single-precision)")))

(event `CheckForShapes`
  (params (InRow :type "Array of Integer") (InCol :type "Array of Integer"))
  ;[1 1 1] Z and T don't work
  (bind _outisi (`self.CheckForI` InRow InCol))
  (if _outisi
    (`KismetSystemLibrary.PrintString` "I")
    (`self.Server_SendID` 0)
    (else
      (bind _outisjorl (`self.CheckForJ` InRow InCol))
      (if _outisjorl
        (bind _outfilterj (`self.FilterForJ` InRow InCol))
        (if _outfilterj
          (`KismetSystemLibrary.PrintString` "J")
          (`self.Server_SendID` 1)
          (else
            (bind _outisjorl_2 (`self.CheckForL` InRow InCol :!label _label))
            (if _outisjorl_2
              (bind _outfilterl (`self.FilterForL` InRow InCol))
              (if _outfilterl
                (`KismetSystemLibrary.PrintString` "L")
                (`self.Server_SendID` 2)
                (else
                  (bind _outist (`self.CheckForT` InRow InCol))
                  (if _outist
                    (`KismetSystemLibrary.PrintString` "T")
                    (`self.Server_SendID` 3)
                    (else
                      (bind _outiso (`self.CheckForO` InRow InCol :!label _label_2))
                      (if _outiso
                        (`KismetSystemLibrary.PrintString` "O")
                        (`self.Server_SendID` 4)
                        (else
                          (bind _outiss (`self.CheckForS` InRow InCol))
                          (if _outiss
                            (`KismetSystemLibrary.PrintString` "S")
                            (`self.Server_SendID` 5)
                            (else
                              (bind _outisz (`self.CheckForZ` InRow InCol))
                              (if _outisz
                                (`KismetSystemLibrary.PrintString` "Z")
                                (`self.Server_SendID` 6)
                                (else
                                  (`KismetSystemLibrary.PrintString` "END")
                                  (`self.Server_SendID` 7)))))))))))
              (else
                (goto _label_2)))))
        (else
          (goto _label)))))
  (set `self.GotResult` true))

(event `CalculateStringAndCount`
  (bind _hitarray (`self.HitArray`))
  (`KismetArrayLibrary.Array_Clear` (`self.rowValues`))
  (`KismetArrayLibrary.Array_Clear` (`self.colValues`))
  (`KismetArrayLibrary.Array_Clear` (`self.RowCountArray`))
  (`self.ResetCounts`)
  (if (`KismetArrayLibrary.Array_IsNotEmpty` _hitarray)
    (for _array_element _hitarray
      (bind _output_get (set `self.currString` (`KismetSystemLibrary.GetObjectName` _array_element)))
      (bind (_lefts _rights) (`KismetStringLibrary.Split` _output_get "-"))
      (`KismetArrayLibrary.Array_Add` (`self.rowValues`) _lefts)
      (`KismetArrayLibrary.Array_Add` (`self.colValues`) _rights))
    (`KismetSystemLibrary.PrintString` "Strings separated")
    (for _array_element_2 (`self.rowValues`)
      (switch `string` _array_element_2
        (:`a`
          (bind _result (`/Engine/EditorBlueprintResources/StandardMacros.IncrementInt` (`self.A_Count`))
            (:`  `
              _)))
        (:`b`
          (bind _result_2 (`/Engine/EditorBlueprintResources/StandardMacros.IncrementInt` (`self.B_Count`))
            (:`  `
              _)))
        (:`c`
          (bind _result_3 (`/Engine/EditorBlueprintResources/StandardMacros.IncrementInt` (`self.C_Count`))
            (:`  `
              _)))
        (:`d`
          (bind _result_4 (`/Engine/EditorBlueprintResources/StandardMacros.IncrementInt` (`self.D_Count`))
            (:`  `
              _)))
        (:`e`
          (bind _result_5 (`/Engine/EditorBlueprintResources/StandardMacros.IncrementInt` (`self.E_Count`))
            (:`  `
              _)))
        (:`f`
          (bind _result_6 (`/Engine/EditorBlueprintResources/StandardMacros.IncrementInt` (`self.F_Count`))
            (:`  `
              _)))
        (:`k`
          (bind _result_7 (`/Engine/EditorBlueprintResources/StandardMacros.IncrementInt` (`self.K_Count`))
            (:`  `
              _)))
        (:`p`
          (bind _result_8 (`/Engine/EditorBlueprintResources/StandardMacros.IncrementInt` (`self.P_Count`))
            (:`  `
              _))))
      (set `self.RowCountArray` (`|MakeArray` _result _result_2 _result_3 _result_4 _result_5 _result_6 _result_7 _result_8)))
    (for _array_element_3 (`self.colValues`)
      (switch `string` _array_element_3
        (:`a`
          (bind _result_9 (`/Engine/EditorBlueprintResources/StandardMacros.IncrementInt` (`self.A_Count`))
            (:`  `
              _)))
        (:`b`
          (bind _result_10 (`/Engine/EditorBlueprintResources/StandardMacros.IncrementInt` (`self.B_Count`))
            (:`  `
              _)))
        (:`c`
          (bind _result_11 (`/Engine/EditorBlueprintResources/StandardMacros.IncrementInt` (`self.C_Count`))
            (:`  `
              _)))
        (:`d`
          (bind _result_12 (`/Engine/EditorBlueprintResources/StandardMacros.IncrementInt` (`self.D_Count`))
            (:`  `
              _)))
        (:`e`
          (bind _result_13 (`/Engine/EditorBlueprintResources/StandardMacros.IncrementInt` (`self.E_Count`))
            (:`  `
              _)))
        (:`f`
          (bind _result_14 (`/Engine/EditorBlueprintResources/StandardMacros.IncrementInt` (`self.F_Count`))
            (:`  `
              _)))
        (:`k`
          (bind _result_15 (`/Engine/EditorBlueprintResources/StandardMacros.IncrementInt` (`self.K_Count`))
            (:`  `
              _)))
        (:`p`
          (bind _result_16 (`/Engine/EditorBlueprintResources/StandardMacros.IncrementInt` (`self.P_Count`))
            (:`  `
              _))))
      (set `self.ColCountArray` (`|MakeArray` _result_9 _result_10 _result_11 _result_12 _result_13 _result_14 _result_15 _result_16)))
    (`self.CheckForShapes` (`self.RowCountArray`) (`self.ColCountArray`))
    (else
      (`KismetSystemLibrary.PrintString` "No click detected"))))

(event `Server_SendID`
  (params (TetrominoID :type Integer))
  (`self.Client_SendID` TetrominoID))

(event `Client_SendID`
  (params (TetrominoID :type Integer))
  (bind _output_get (set `self.TetrominoID` TetrominoID))
  (bind _asbp_blockrun_gm (cast `/Game/_USER/Moz/Blueprints/BP_BlockrunGM` (`GameplayStatics.GetGameMode`)))
  (`/Game/_USER/Moz/Blueprints/BP_BlockrunGM.SetTetroID` _asbp_blockrun_gm _output_get))

(event `ResetCounts`
  (set `self.A_Count` 0)
  (set `self.B_Count` 0)
  (set `self.C_Count` 0)
  (set `self.D_Count` 0)
  (set `self.E_Count` 0)
  (set `self.F_Count` 0)
  (set `self.K_Count` 0)
  (set `self.P_Count` 0))

(event `AfterLock`
  (bind _currentplayercontroller (`self.CurrentPlayerController`))
  ;[1 1 1] When shape is locked in
  (`self.ResetCounts`)
  (if (`self.GotResult`)
    (`/Game/_USER/Moz/Blueprints/BP_BlockrunController.Server_SetSpawnTransform` _currentplayercontroller (`/Game/_USER/Moz/Blueprints/BP_BlockrunController.ReturnZoneLoc` _currentplayercontroller))
    (`/Game/_USER/Moz/Blueprints/BP_BlockrunController.Server_SpawnToLocation` _currentplayercontroller false)
    (bind _asbp_blockrun_char_f (cast `/Game/_USER/Moz/Blueprints/Character/BP_BlockrunCharF` (`Controller.K2_GetPawn` _currentplayercontroller)))
    (`/Game/_USER/Moz/Blueprints/Character/BP_BlockrunCharF.SwitchToThirdPerson` _asbp_blockrun_char_f)
    (set `self.GotResult` false)
    (`self.K2_DestroyActor`)
    (`GameplayStatics.UnloadStreamLevelBySoftObjectPtr` (`/Game/_USER/Moz/Blueprints/Objects/BP_DoorDummy.LevelToLoad` (`/Game/_USER/Moz/Blueprints/BP_BlockrunController.CurrentDummyDoorRef` _currentplayercontroller)))))

(fn `CheckForI`
  (params (InRowArray :type "Array of Integer") (InColArray :type "Array of Integer"))
  (returns (OutIsI :type Boolean))
  (return (or (`KismetArrayLibrary.Array_Contains` InRowArray 4) (`KismetArrayLibrary.Array_Contains` InColArray 4))))

(fn `CheckForJ`
  (params (InRowArray :type "Array of Integer") (InColArray :type "Array of Integer"))
  (returns (OutIsJorL :type Boolean))
  (bind _returnvalue (`KismetArrayLibrary.Array_Find` InRowArray 3))
  (bind _returnvalue_2 (`KismetArrayLibrary.Array_Find` InColArray 2))
  (bind _returnvalue_3 (`KismetArrayLibrary.Array_Find` InRowArray 2))
  (bind _returnvalue_4 (`KismetArrayLibrary.Array_Find` InColArray 3))
  (bind _returnvalue_5 (`KismetArrayLibrary.Array_Find` InRowArray 3))
  (bind _returnvalue_6 (`KismetArrayLibrary.Array_Find` InColArray 2))
  (bind _returnvalue_7 (`KismetArrayLibrary.Array_Find` InRowArray 2))
  (bind _returnvalue_8 (`KismetArrayLibrary.Array_Find` InColArray 3))
  (return (or (and (`KismetArrayLibrary.Array_Contains` InRowArray 3) (`KismetArrayLibrary.Array_Contains` InColArray 2)) (and (and (> _returnvalue 4) (> _returnvalue (`KismetArrayLibrary.Array_Find` InRowArray 1))) (or (== _returnvalue_2 3) (== _returnvalue_2 4))) (and (and (or (== _returnvalue_5 0) (> _returnvalue_5 4)) (< _returnvalue_5 (`KismetArrayLibrary.Array_Find` InRowArray 1))) (or (== _returnvalue_6 1) (== _returnvalue_6 2))) (and (and (< _returnvalue_4 5) (> _returnvalue_4 (`KismetArrayLibrary.Array_Find` InColArray 1))) (or (== _returnvalue_3 0) (== _returnvalue_3 5))) (and (and (< _returnvalue_8 4) (< _returnvalue_8 (`KismetArrayLibrary.Array_Find` InColArray 1))) (or (== _returnvalue_7 6) (== _returnvalue_7 7))))))

(fn `CheckForL`
  (params (InRowArray :type "Array of Integer") (InColArray :type "Array of Integer"))
  (returns (OutIsJorL :type Boolean))
  (bind _returnvalue (`KismetArrayLibrary.Array_Find` InRowArray 3))
  (bind _returnvalue_2 (`KismetArrayLibrary.Array_Find` InColArray 2))
  (bind _returnvalue_3 (`KismetArrayLibrary.Array_Find` InRowArray 2))
  (bind _returnvalue_4 (`KismetArrayLibrary.Array_Find` InColArray 3))
  (bind _returnvalue_5 (`KismetArrayLibrary.Array_Find` InRowArray 3))
  (bind _returnvalue_6 (`KismetArrayLibrary.Array_Find` InColArray 2))
  (bind _returnvalue_7 (`KismetArrayLibrary.Array_Find` InRowArray 2))
  (bind _returnvalue_8 (`KismetArrayLibrary.Array_Find` InColArray 3))
  (return (or (and (`KismetArrayLibrary.Array_Contains` InRowArray 3) (`KismetArrayLibrary.Array_Contains` InColArray 2)) (and (and (> _returnvalue 4) (> _returnvalue (`KismetArrayLibrary.Array_Find` InRowArray 1))) (or (== _returnvalue_2 1) (== _returnvalue_2 2))) (and (and (or (== _returnvalue_5 0) (> _returnvalue_5 4)) (< _returnvalue_5 (`KismetArrayLibrary.Array_Find` InRowArray 1))) (or (== _returnvalue_6 3) (== _returnvalue_6 4))) (and (and (< _returnvalue_4 5) (> _returnvalue_4 (`KismetArrayLibrary.Array_Find` InColArray 1))) (or (== _returnvalue_3 6) (== _returnvalue_3 7))) (and (and (< _returnvalue_8 4) (< _returnvalue_8 (`KismetArrayLibrary.Array_Find` InColArray 1))) (or (== _returnvalue_7 0) (== _returnvalue_7 5))))))

(fn `CheckForO`
  (params (InRowArray :type "Array of Integer") (InColArray :type "Array of Integer"))
  (returns (OutIsO :type Boolean))
  (locals (localRowsOnlyTwos :type Boolean) (localColumnsOnlyTwos :type Boolean))
  (for _array_element InRowArray
    (if (== (mod _array_element 2) 0)
      (set `local.localRowsOnlyTwos` true)
      (for _array_element_2 InColArray
        (if (== (mod _array_element_2 2) 0)
          (set `local.localColumnsOnlyTwos` true)
          (else
            (set `local.localColumnsOnlyTwos` false)
            (break))))
      (return (and (`local.localRowsOnlyTwos`) (`local.localColumnsOnlyTwos`)))
      (else
        (set `local.localRowsOnlyTwos` false)
        (break)))))

(fn `CheckForS`
  (params (InRowArray :type "Array of Integer") (InColArray :type "Array of Integer"))
  (returns (OutIsS :type Boolean))
  (locals (localOnlyTwoInRow :type Boolean) (localTwoInBetweenOnes :type Boolean))
  (bind _returnvalue (`KismetArrayLibrary.Array_Find` InColArray 2))
  (for _array_element InRowArray
    (if (== (mod _array_element 2) 0)
      (set `local.localOnlyTwoInRow` true)
      (else
        (set `local.localOnlyTwoInRow` false))))
  (bind _result (`/Engine/EditorBlueprintResources/StandardMacros.DecrementInt` _returnvalue)
    (:`  `
      (bind _result_2 (`/Engine/EditorBlueprintResources/StandardMacros.IncrementInt` _returnvalue)
        (:`  `
          (if (and (== (`|GetArrayItem` InColArray _result) 1) (== (`|GetArrayItem` InColArray _result_2) 1))
            (set `local.localTwoInBetweenOnes` true)
            (else
              (set `local.localTwoInBetweenOnes` false)))
          (return (and (`local.localOnlyTwoInRow`) (`local.localOnlyTwoInRow`))))))))

(fn `CheckForT`
  (params (InRowArray :type "Array of Integer") (InColArray :type "Array of Integer"))
  (returns (OutIsT :type Boolean))
  (bind _returnvalue (`KismetArrayLibrary.Array_Find` InColArray 2))
  (bind _returnvalue_2 (`KismetArrayLibrary.Array_Find` InRowArray 3))
  (bind _returnvalue_3 (`KismetArrayLibrary.Array_Find` InColArray 2))
  (bind _returnvalue_4 (`KismetArrayLibrary.Array_Find` InRowArray 2))
  (bind _returnvalue_5 (`KismetArrayLibrary.Array_Find` InColArray 3))
  (bind _returnvalue_6 (`KismetArrayLibrary.Array_Find` InRowArray 3))
  (bind _returnvalue_7 (`KismetArrayLibrary.Array_Find` InRowArray 2))
  (bind _returnvalue_8 (`KismetArrayLibrary.Array_Find` InColArray 3))
  (return (or (and (`KismetArrayLibrary.Array_Contains` InRowArray 3) (`KismetArrayLibrary.Array_Contains` InColArray 2)) (and (and (> _returnvalue_2 4) (> _returnvalue_2 (`KismetArrayLibrary.Array_Find` InRowArray 1))) (and (== (`|GetArrayItem` InColArray (`KismetMathLibrary.Clamp` (- _returnvalue 1) 0 7)) 1) (== (`|GetArrayItem` InColArray (`KismetMathLibrary.Clamp` (+ _returnvalue 1) 0 7)) 1))) (and (and (or (== _returnvalue_6 0) (> _returnvalue_6 4)) (< _returnvalue_6 (`KismetArrayLibrary.Array_Find` InRowArray 1))) (and (== (`|GetArrayItem` InRowArray (`KismetMathLibrary.Clamp` (- _returnvalue_3 1) 0 7)) 1) (== (`|GetArrayItem` InRowArray (`KismetMathLibrary.Clamp` (+ _returnvalue_3 1) 0 7)) 1))) (and (and (< _returnvalue_5 5) (> _returnvalue_5 (`KismetArrayLibrary.Array_Find` InColArray 1))) (or (== _returnvalue_4 5) (== _returnvalue_4 6))) (and (and (< _returnvalue_8 4) (< _returnvalue_8 (`KismetArrayLibrary.Array_Find` InColArray 1))) (or (== _returnvalue_7 5) (== _returnvalue_7 6))))))

(fn `CheckForZ`
  (params (InRowArray :type "Array of Integer") (InColArray :type "Array of Integer"))
  (returns (OutIsZ :type Boolean))
  (locals (localOnlyTwoInRow :type Boolean) (localTwoInBetweenOnes :type Boolean))
  (bind _returnvalue (`KismetArrayLibrary.Array_Find` InColArray 2))
  ;[1 1 1] Need to fix; give same OP as Check for S
  (for _array_element InRowArray
    (if (== (mod _array_element 2) 0)
      (set `local.localOnlyTwoInRow` true)
      (else
        (set `local.localOnlyTwoInRow` false))))
  (bind _result (`/Engine/EditorBlueprintResources/StandardMacros.DecrementInt` _returnvalue)
    (:`  `
      (bind _result_2 (`/Engine/EditorBlueprintResources/StandardMacros.IncrementInt` _returnvalue)
        (:`  `
          (if (and (== (`|GetArrayItem` InColArray _result) 1) (== (`|GetArrayItem` InColArray _result_2) 1))
            (set `local.localTwoInBetweenOnes` true)
            (else
              (set `local.localTwoInBetweenOnes` false)))
          (return (and (`local.localOnlyTwoInRow`) (`local.localOnlyTwoInRow`))))))))

(fn `FilterForJ`
  (params (InRowArray :type "Array of Integer") (InColArray :type "Array of Integer"))
  (returns (OutFilterJ :type Boolean))
  (return (or (and (< (`KismetArrayLibrary.Array_Find` InRowArray 3) (`KismetArrayLibrary.Array_Find` InRowArray 1)) (< (`KismetArrayLibrary.Array_Find` InColArray 2) (`KismetArrayLibrary.Array_Find` InColArray 1))) (and (< (`KismetArrayLibrary.Array_Find` InRowArray 1) (`KismetArrayLibrary.Array_Find` InRowArray 3)) (< (`KismetArrayLibrary.Array_Find` InColArray 1) (`KismetArrayLibrary.Array_Find` InColArray 2))))))

(fn `FilterForL`
  (params (InRowArray :type "Array of Integer") (InColArray :type "Array of Integer"))
  (returns (OutFilterL :type Boolean))
  (return (or (and (< (`KismetArrayLibrary.Array_Find` InRowArray 3) (`KismetArrayLibrary.Array_Find` InRowArray 1)) (< (`KismetArrayLibrary.Array_Find` InColArray 1) (`KismetArrayLibrary.Array_Find` InColArray 2))) (and (< (`KismetArrayLibrary.Array_Find` InRowArray 2) (`KismetArrayLibrary.Array_Find` InRowArray 1)) (< (`KismetArrayLibrary.Array_Find` InColArray 3) (`KismetArrayLibrary.Array_Find` InColArray 1))) (and (< (`KismetArrayLibrary.Array_Find` InRowArray 1) (`KismetArrayLibrary.Array_Find` InRowArray 3)) (< (`KismetArrayLibrary.Array_Find` InColArray 2) (`KismetArrayLibrary.Array_Find` InColArray 1))) (and (< (`KismetArrayLibrary.Array_Find` InRowArray 1) (`KismetArrayLibrary.Array_Find` InRowArray 2)) (< (`KismetArrayLibrary.Array_Find` InColArray 1) (`KismetArrayLibrary.Array_Find` InColArray 3))))))

(fn `GenerateString`
  (params (InComponents :type "Array of PrimitiveComponent Object Reference"))
  (returns (ReturnString :type String))
  (for _array_element InComponents
    (bind _output_get (set `self.currString` (`KismetSystemLibrary.GetObjectName` _array_element)))
    (bind (_lefts _rights) (`KismetStringLibrary.Split` _output_get "-"))
    (`KismetArrayLibrary.Array_Add` (`self.rowValues`) _lefts)
    (`KismetArrayLibrary.Array_Add` (`self.colValues`) _rights))
  (bind _output_get_2 (set `self.overallString` (`KismetStringLibrary.Concat_StrStr` (`self.overallString`) (`self.currString`))))
  (return _output_get_2))

(fn `UserConstructionScript`
  (`KismetArrayLibrary.Array_Clear` (`self.ComponentArray`))
  (for _array_element (`SceneComponent.GetChildrenComponents` (`self.DefaultSceneRoot`) false)
    (bind _asstatic_mesh_component (cast `StaticMeshComponent` _array_element))
    (`KismetArrayLibrary.Array_AddUnique` (`self.ComponentArray`) _asstatic_mesh_component)))