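; Player controller for the main menu level that brings up the menu when play begins.
; For the local controller, BeginPlay creates and displays the WB_MainMenu widget and shows the mouse cursor.
; It then casts the game instance to BP_CustomGameInstance and calls its SpawnCharacter.
; An older, disconnected branch using WBP_MainMenu remains but never runs.
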(event `self.ReceiveBeginPlay`
  (if (`self.IsLocalPlayerController`)
    ;[1 1 1] Create Main Menu Widget
    (bind _returnvalue (`|CreateWidget` "/Game/Multiplayer/Widgets/MainMenu/WB_MainMenu.WB_MainMenu_C" self))
    (`UserWidget.AddToViewport` _returnvalue 0)
    (set `self.bShowMouseCursor` true)
    (bind _asbp_custom_game_instance (cast `/Game/_USER/Moz/Blueprints/BP_CustomGameInstance` (`GameplayStatics.GetGameInstance`)))
    (`/Game/_USER/Moz/Blueprints/BP_CustomGameInstance.SpawnCharacter` _asbp_custom_game_instance)))

(fn `UserConstructionScript`)