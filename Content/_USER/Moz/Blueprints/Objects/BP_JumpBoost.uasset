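; BP_JumpBoost is a pickup that temporarily raises the jump velocity of an overlapping BP_BlockrunCharF.
; On sphere overlap it flags and tints the boost indicator through BP_BlockrunController, sets the new velocity, hides itself and plays a sound.
; One cooldown delay times both respawn and boost expiry, restoring a hardcoded default jump velocity.
; The construction script toggles its text label; other character types get the controller feedback but no boost.
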(event `self.COLL_Sphere.OnComponentBeginOverlap`
  (params (OverlappedComponent :type "PrimitiveComponent Object Reference") (OtherActor :type "Actor Object Reference") (OtherComp :type "PrimitiveComponent Object Reference") (OtherBodyIndex :type Integer) (bFromSweep :type Boolean) (SweepResult :type "HitResult Structure (by ref)"))
  ;[1 1 1] When CharF overlaps with this BP, then activate jump boost, hide the powerup (for 3 sec) and then spawn it back
  (bind _asbp_blockrun_controller (cast `/Game/_USER/Moz/Blueprints/BP_BlockrunController` (`self.GetInstigatorController` OtherActor)))
  (`/Game/_USER/Moz/Blueprints/BP_BlockrunController.Client_SetJumpBoostFlag` _asbp_blockrun_controller true)
  (`/Game/_USER/Moz/Blueprints/BP_BlockrunController.Client_SetColorAndOpacity` _asbp_blockrun_controller (struct :`G` 0.795267 :`B` 1.0 :`A` 1.0))
  ;;[1 1 1] Only works for one type of Char. TODO: Change logic for multiple char (via Cast Failed)
  (bind _asbp_blockrun_char_f (cast `/Game/_USER/Moz/Blueprints/Character/BP_BlockrunCharF` OtherActor))
  (bind _charactermovement (`Character.CharacterMovement` _asbp_blockrun_char_f))
  (set `CharacterMovementComponent.JumpZVelocity` (`self.NewJumpVelocity`) _charactermovement)
  (`self.SetActorHiddenInGame` self true)
  (`PrimitiveComponent.SetCollisionEnabled` (`self.COLL_Sphere`) "NoCollision")
  (`GameplayStatics.PlaySoundAtLocation` "/Engine/VREditor/Sounds/UI/Object_PickUp.Object_PickUp" (`self.K2_GetActorLocation`) (struct) 1.0 1.0 0.0 null null null null)
  (`KismetSystemLibrary.Delay` (`self.CooldownTime`))
  (`self.SetActorHiddenInGame` self false)
  (`PrimitiveComponent.SetCollisionEnabled` (`self.COLL_Sphere`) "QueryOnly")
  (`/Engine/EditorBlueprintResources/StandardMacros.IsValid` _asbp_blockrun_char_f
    (:`Is Valid`
      (set `CharacterMovementComponent.JumpZVelocity` 600.0 _charactermovement)
      (`/Game/_USER/Moz/Blueprints/BP_BlockrunController.Client_SetJumpBoostFlag` _asbp_blockrun_controller false)
      (`/Game/_USER/Moz/Blueprints/BP_BlockrunController.Client_SetColorAndOpacity` _asbp_blockrun_controller (struct :`R` 1.0 :`G` 1.0 :`B` 1.0 :`A` 0.5)))))

(fn `UserConstructionScript`
  (if (`self.DisplayText`)
    (`SceneComponent.SetVisibility` (`self.TXT_JumpBoost`) true false)
    (else
      (`SceneComponent.SetVisibility` (`self.TXT_JumpBoost`) false false))))