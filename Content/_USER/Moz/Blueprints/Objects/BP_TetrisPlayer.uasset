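; BP_TetrisPlayer is a trigger object that switches an overlapping BP_BlockrunCharF player's input to Tetris controls.
; Its Box overlap calls a client context-change event with the other actor and prints a display name.
; That event reaches the controlled pawn through the instigator controller, then uses the controller's Enhanced Input user settings to replace the character's current mapping context with IMC_TetrisPlayer.
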(event `self.Box.OnComponentBeginOverlap`
  (params (OverlappedComponent :type "PrimitiveComponent Object Reference") (OtherActor :type "Actor Object Reference") (OtherComp :type "PrimitiveComponent Object Reference") (OtherBodyIndex :type Integer) (bFromSweep :type Boolean) (SweepResult :type "HitResult Structure (by ref)"))
  (`self.Client_ChangeContext` OtherActor)
  (`KismetSystemLibrary.PrintString` (`KismetSystemLibrary.GetDisplayName` null)))

(event `Client_ChangeContext`
  (params (Target :type "Actor Object Reference"))
  (bind _returnvalue (`self.GetInstigatorController` Target))
  (bind _asbp_blockrun_char_f (cast `/Game/_USER/Moz/Blueprints/Character/BP_BlockrunCharF` (`Controller.K2_GetPawn` _returnvalue)))
  (bind _returnvalue_2 (message `EnhancedInputSubsystemInterface.GetUserSettings` _returnvalue))
  (message `EnhancedInputSubsystemInterface.RemoveMappingContext` _returnvalue_2 (`/Game/_USER/Moz/Blueprints/Character/BP_BlockrunCharF.CurrentMappingContext` _asbp_blockrun_char_f) (struct))
  (message `EnhancedInputSubsystemInterface.AddMappingContext` _returnvalue_2 "/Game/_USER/Moz/Blueprints/Input/Tetris/IMC_TetrisPlayer.IMC_TetrisPlayer" 0 (struct)))

(fn `UserConstructionScript`)