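; BP_Key is a key pickup that only the puzzle player can collect.
; On sphere overlap, a puzzle player's controller is passed to a server event that calls its key update, then the key plays a click and destroys itself.
; Other players see a Denied HUD widget for a few seconds.
; The construction script optionally shows the key's name as a text label.
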(event `self.COLL_Sphere.OnComponentBeginOverlap`
  (params (OverlappedComponent :type "PrimitiveComponent Object Reference") (OtherActor :type "Actor Object Reference") (OtherComp :type "PrimitiveComponent Object Reference") (OtherBodyIndex :type Integer) (bFromSweep :type Boolean) (SweepResult :type "HitResult Structure (by ref)"))
  (bind _returnvalue (`self.GetInstigatorController` OtherActor))
  ;[1 1 1] On overlap, tell server to give key to the player that overlapped
  (bind _asbp_blockrun_controller (cast `/Game/_USER/Moz/Blueprints/BP_BlockrunController` _returnvalue))
  (if (`/Game/_USER/Moz/Blueprints/BP_BlockrunController.IsPuzzlePlayer` _asbp_blockrun_controller)
    (`self.Server_GiveKeyToPlayer` _returnvalue)
    (`GameplayStatics.PlaySoundAtLocation` "/Engine/VREditor/Sounds/VR_click3.VR_click3" (`self.K2_GetActorLocation`) (struct) 1.0 1.0 0.0 null null null null)
    (`self.K2_DestroyActor`)
    (else
      (bind _wbp_denied (`/Game/_USER/Moz/Blueprints/Widgets/WBP_MainHUD.WBP_Denied` (`/Game/_USER/Moz/Blueprints/BP_BlockrunController.MainHUDRef` _asbp_blockrun_controller)))
      (`Widget.SetVisibility` _wbp_denied "Visible")
      (`KismetSystemLibrary.Delay` 3.0)
      (`Widget.SetVisibility` _wbp_denied "Hidden"))))

(event `Server_GiveKeyToPlayer`
  (params (InController :type "Controller Object Reference"))
  ;[1 1 1] Whatever player the server has determined that has picked up, call its local Update Key function
  (bind _asbp_blockrun_controller (cast `/Game/_USER/Moz/Blueprints/BP_BlockrunController` InController))
  (`/Game/_USER/Moz/Blueprints/BP_BlockrunController.Server_UpdateKey` _asbp_blockrun_controller true))

(fn `UserConstructionScript`
  (locals (localEntityName :type Text :default "NSLOCTEXT(\"\", \"50D156014DA2B42C87C13E9D112C4B78\", \"Key\")"))
  (bind _txt_collectiblename (`self.TXT_CollectibleName`))
  (if (`self.TextVisible`)
    (`SceneComponent.SetVisibility` _txt_collectiblename true false)
    (`TextRenderComponent.K2_SetText` _txt_collectiblename (`local.localEntityName`))
    (else
      (`SceneComponent.SetVisibility` _txt_collectiblename false false))))