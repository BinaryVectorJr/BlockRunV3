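; BP_RowSpawnedEntity is an actor that eases vertically toward a TargetZ height and removes itself when it has no supporting block.
; TargetZ starts at the spawn height, and Tick lerps halfway toward it each frame until nearly equal.
; Once settled, it line-traces 50 units along negative Y every frame and destroys itself unless the hit actor's class is exactly BP_BaseSingleBlock.
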(event `self.ReceiveBeginPlay`
  (bind (_returnvalue_x _returnvalue_y _returnvalue_z) (`KismetMathLibrary.BreakVector` (`self.K2_GetActorLocation`)))
  (set `self.TargetZ` _returnvalue_z))

(event `self.ReceiveTick`
  (params (DeltaSeconds :type "Float (single-precision)"))
  (bind (_returnvalue_x _returnvalue_y _returnvalue_z) (`KismetMathLibrary.BreakVector` (`self.K2_GetActorLocation`)))
  (bind _returnvalue (`self.K2_GetActorLocation`))
  (bind (_returnvalue_x_2 _returnvalue_y_2 _returnvalue_z_2) (`KismetMathLibrary.BreakVector` (`self.K2_GetActorLocation`)))
  ;[1 1 1] Update position on tick
  (if (`KismetMathLibrary.NearlyEqual_FloatFloat` (`self.TargetZ`) _returnvalue_z_2 0.1)
    ;[1 1 1] If nothing is detected undeneath, then destroy this actor
    (bind _outhit (`KismetSystemLibrary.LineTraceSingle` _returnvalue (- _returnvalue (0.0 50.0 0.0)) "TraceTypeQuery1"))
    (if (not (== (`GameplayStatics.GetObjectClass` (`.HitActor` (`GameplayStatics.BreakHitResult` _outhit))) "/Game/_USER/Moz/Blueprints/Tetromino/BP_BaseSingleBlock.BP_BaseSingleBlock_C"))
      (`self.K2_DestroyActor`))
    (else
      (`self.K2_SetActorLocation` (`KismetMathLibrary.MakeVector` _returnvalue_x _returnvalue_y (`KismetMathLibrary.Lerp` _returnvalue_z (`self.TargetZ`) 0.5))))))

(fn `UserConstructionScript`)