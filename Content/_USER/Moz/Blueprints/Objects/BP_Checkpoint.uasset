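; BP_Checkpoint is a one-time checkpoint actor that updates a player's spawn point when touched.
; The first sphere overlap latches it activated and recolors the button mesh blue through a dynamic material instance.
; It then casts the overlapper's instigator controller to BP_BlockrunController, calls ServerSetSpawnTransform with PSCheckpointTransform's location and rotation, and plays a sound.
; The latch precedes the cast, so any overlapping actor consumes the checkpoint.
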(event `self.COLL_Sphere.OnComponentBeginOverlap`
  (params (OverlappedComponent :type "PrimitiveComponent Object Reference") (OtherActor :type "Actor Object Reference") (OtherComp :type "PrimitiveComponent Object Reference") (OtherBodyIndex :type Integer) (bFromSweep :type Boolean) (SweepResult :type "HitResult Structure (by ref)"))
  (bind _sm_button (`self.SM_Button`))
  (bind (_returnvalue_location _returnvalue_rotation) (`KismetMathLibrary.BreakTransform` (`SceneComponent.K2_GetComponentToWorld` (`self.PS_CheckpointTransform`))))
  (if (not (`self.IsCheckpointActivated`))
    (set `self.IsCheckpointActivated` true)
    (bind _returnvalue (`PrimitiveComponent.CreateDynamicMaterialInstance` _sm_button 0 (`PrimitiveComponent.GetMaterial` _sm_button 0) "None"))
    (bind _output_get (set `self.DynamicMaterialInstance` _returnvalue))
    (`MaterialInstanceDynamic.SetVectorParameterValue` _output_get "BaseColorVector" (struct :`B` 0.75 :`A` 1.0))
    (bind _asbp_blockrun_controller (cast `/Game/_USER/Moz/Blueprints/BP_BlockrunController` (`self.GetInstigatorController` OtherActor)))
    (`/Game/_USER/Moz/Blueprints/BP_BlockrunController.Server_SetSpawnTransform` _asbp_blockrun_controller (`KismetMathLibrary.MakeTransform` _returnvalue_location _returnvalue_rotation))
    (`GameplayStatics.PlaySoundAtLocation` "/Engine/VREditor/Sounds/UI/Leave_Simulate.Leave_Simulate" (`self.K2_GetActorLocation`) (struct) 1.0 1.0 0.0 null null null null)))

(fn `UserConstructionScript`)