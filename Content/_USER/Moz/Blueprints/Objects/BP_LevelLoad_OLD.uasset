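; BP_LevelLoad_OLD is a trigger actor that handles level streaming and player relocation through entry and exit boxes.
; Any overlap on EntryBox asynchronously loads LevelToLoad, while a separate UnloadLevel event unloads LevelToUnload.
; ExitBox has the overlapping actor's BP_BlockrunController set its spawn transform to the Sphere and respawn there via server calls.
; A PlayerHasEnteredZone rep-notify flags EnteredController as a puzzle player.
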(event `self.EntryBox.OnComponentBeginOverlap`
  (params (OverlappedComponent :type "PrimitiveComponent Object Reference") (OtherActor :type "Actor Object Reference") (OtherComp :type "PrimitiveComponent Object Reference") (OtherBodyIndex :type Integer) (bFromSweep :type Boolean) (SweepResult :type "HitResult Structure (by ref)"))
  (`GameplayStatics.LoadStreamLevel` (`self.LevelToLoad`) true))

(event `self.ExitBox.OnComponentBeginOverlap`
  (params (OverlappedComponent :type "PrimitiveComponent Object Reference") (OtherActor :type "Actor Object Reference") (OtherComp :type "PrimitiveComponent Object Reference") (OtherBodyIndex :type Integer) (bFromSweep :type Boolean) (SweepResult :type "HitResult Structure (by ref)"))
  (bind _sphere (`self.Sphere`))
  (bind _asbp_blockrun_controller (cast `/Game/_USER/Moz/Blueprints/BP_BlockrunController` (`self.GetInstigatorController` OtherActor))
    (:`then`
      (`/Game/_USER/Moz/Blueprints/BP_BlockrunController.Server_SetSpawnTransform` _asbp_blockrun_controller (`KismetMathLibrary.MakeTransform` (`SceneComponent.K2_GetComponentLocation` _sphere) (`SceneComponent.K2_GetComponentRotation` _sphere)))
      (`KismetSystemLibrary.PrintString` "Set in place")
      (`/Game/_USER/Moz/Blueprints/BP_BlockrunController.Server_SpawnToLocation` _asbp_blockrun_controller))
    (:`CastFailed`
      (`KismetSystemLibrary.PrintString` "Failed setting"))))

(event `UnloadLevel`
  (`GameplayStatics.UnloadStreamLevel` (`self.LevelToUnload`)))

(fn `OnRep_PlayerHasEnteredZone`
  (set `/Game/_USER/Moz/Blueprints/BP_BlockrunController.IsPuzzlePlayer` true (`self.EnteredController`)))

(fn `UserConstructionScript`)