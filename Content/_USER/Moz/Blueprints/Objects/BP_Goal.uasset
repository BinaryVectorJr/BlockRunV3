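; BP_Goal is a goal marker actor that, when flagged IsEndGoal, notifies a Blockrun player's controller that the goal has been reached.
; In that case, the construction script shows a statue mesh with collision disabled and sets the end-goal text.
; A capsule overlap casts the overlapping actor's instigator controller to BP_BlockrunController and calls ClientReachGoal.
; When the flag is off, neither script does anything.
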(event `self.COLL_Capsule.OnComponentBeginOverlap`
  (params (OverlappedComponent :type "PrimitiveComponent Object Reference") (OtherActor :type "Actor Object Reference") (OtherComp :type "PrimitiveComponent Object Reference") (OtherBodyIndex :type Integer) (bFromSweep :type Boolean) (SweepResult :type "HitResult Structure (by ref)"))
  (if (`self.IsEndGoal`)
    (bind _asbp_blockrun_controller (cast `/Game/_USER/Moz/Blueprints/BP_BlockrunController` (`self.GetInstigatorController` OtherActor)))
    (`/Game/_USER/Moz/Blueprints/BP_BlockrunController.Client_ReachGoal` _asbp_blockrun_controller)))

(fn `UserConstructionScript`
  (locals (localEndGoalText :type Text :default "NSLOCTEXT(\"\", \"B8DDF8884EEC8A397AFF5B9478A11BCA\", \"Goal\")"))
  (bind _staticmesh (`self.StaticMesh`))
  (if (`self.IsEndGoal`)
    (`StaticMeshComponent.SetStaticMesh` _staticmesh "/Game/StarterContent/Props/SM_Statue.SM_Statue")
    (`PrimitiveComponent.SetCollisionEnabled` _staticmesh "NoCollision")
    (`TextRenderComponent.K2_SetText` (`self.TextRender`) (`local.localEndGoalText`))))