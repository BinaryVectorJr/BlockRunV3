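; Networked key-locked door that also serves as a transition into a streamed level.
; Server-side entry box overlaps call the player's BP_BlockrunController to drive door logic and the locked message.
; OpenDoor consumes the key once, and multicast events animate opening and closing with timelines.
; A loader box streams LevelToLoad for the local player, stores a return point and requests a server teleport, optionally showing a brief loading widget.
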(event `self.COLL_EntryBox.OnComponentBeginOverlap`
  (params (OverlappedComponent :type "PrimitiveComponent Object Reference") (OtherActor :type "Actor Object Reference") (OtherComp :type "PrimitiveComponent Object Reference") (OtherBodyIndex :type Integer) (bFromSweep :type Boolean) (SweepResult :type "HitResult Structure (by ref)"))
  (`/Engine/EditorBlueprintResources/ActorMacros.Switch Has Authority`
    (:`Authority`
      (if (not (`self.IsDoorOpen`))
        (bind _asbp_blockrun_controller (cast `/Game/_USER/Moz/Blueprints/BP_BlockrunController` (`self.GetInstigatorController` OtherActor)))
        (if (`/Game/_USER/Moz/Blueprints/BP_BlockrunController.HasKey` _asbp_blockrun_controller)
          ;[1 1 1] If has key, tell server to call client's Door Logic fn (This can seem redundant, but if you want the door to do something else, then code can go here)
          (`/Game/_USER/Moz/Blueprints/BP_BlockrunController.Server_ControlDoorLogic` _asbp_blockrun_controller true self)
          (else
            ;[1 1 1] If doesnt have key still server will tell the PC to call the door control logic (but the llogic will change once the function is called)
            (`/Game/_USER/Moz/Blueprints/BP_BlockrunController.Server_ControlDoorLogic` _asbp_blockrun_controller true self)))))))

(event `self.COLL_EntryBox.OnComponentEndOverlap`
  (params (OverlappedComponent :type "PrimitiveComponent Object Reference") (OtherActor :type "Actor Object Reference") (OtherComp :type "PrimitiveComponent Object Reference") (OtherBodyIndex :type Integer))
  ;[1 1 1] Once player leaves door zone, reset the LOCKED text by setting show text bool to false
  (`/Engine/EditorBlueprintResources/ActorMacros.Switch Has Authority`
    (:`Authority`
      (bind _asbp_blockrun_controller (cast `/Game/_USER/Moz/Blueprints/BP_BlockrunController` (`self.GetInstigatorController` OtherActor)))
      (`/Game/_USER/Moz/Blueprints/BP_BlockrunController.Server_ControlDoorLogic` _asbp_blockrun_controller false self))))

(event `OpenDoor`
  (params (InPlayerController :type "/Game/_USER/Moz/Blueprints/BP_BlockrunController Object Reference"))
  ;[1 1 1] Server fn to call updation of key (when used), set the opening of door to be true and then opening of door (multi replicate event)
  (if (`/Game/_USER/Moz/Blueprints/BP_BlockrunController.HasKey` InPlayerController)
    (`/Engine/EditorBlueprintResources/StandardMacros.DoOnce` false
      (:`Completed`
        (`/Game/_USER/Moz/Blueprints/BP_BlockrunController.Server_UpdateKey` InPlayerController false)
        (set `self.IsDoorOpen` true)
        (`self.Multi_DoorOpenEvent`)))))

(event `Multi_DoorOpenEvent`
  ;[1 1 1] Multi replicate fn (shows on server and client) for opening the door (visually)
  (`GameplayStatics.PlaySoundAtLocation` "/Engine/EditorSounds/GamePreview/EndSimulate.EndSimulate" (`self.K2_GetActorLocation`) (struct) 1.0 1.0 0.0 null null null null)
  (bind (_direction _dooropenrot) (`Timeline|DoorOpen` :!via `PlayFromStart`)
    (:`Update`
      (`SceneComponent.K2_SetRelativeRotation` (`self.SM_Door`) (`KismetMathLibrary.MakeRotator` 0.0 0.0 (`KismetMathLibrary.Lerp` 180.0 90.0 _dooropenrot)) false false))))

(event `CloseDoor`
  (params (InPlayerController :type "/Game/_USER/Moz/Blueprints/BP_BlockrunController Object Reference"))
  ;[1 1 1] Server call to close door
  (set `self.IsDoorOpen` false)
  (`self.Multi_DoorCloseEvent` InPlayerController))

(event `Multi_DoorCloseEvent`
  (params (InPlayerController :type "/Game/_USER/Moz/Blueprints/BP_BlockrunController Object Reference"))
  ;[1 1 1] Multi replicate fn (shows on server and client) for closing the door (visually)
  (bind (_direction _dooropenrot) (`Timeline|Timeline` :!via `PlayFromStart`)
    (:`Update`
      (`SceneComponent.K2_SetRelativeRotation` (`self.SM_Door`) (`KismetMathLibrary.MakeRotator` 0.0 0.0 (`KismetMathLibrary.Lerp` 90.0 180.0 _dooropenrot)) false false)
      (`/Game/_USER/Moz/Blueprints/BP_BlockrunController.Server_ControlDoorLogic` InPlayerController false self))))

(event `self.COLL_LevelLoader.OnComponentBeginOverlap`
  (params (OverlappedComponent :type "PrimitiveComponent Object Reference") (OtherActor :type "Actor Object Reference") (OtherComp :type "PrimitiveComponent Object Reference") (OtherBodyIndex :type Integer) (bFromSweep :type Boolean) (SweepResult :type "HitResult Structure (by ref)"))
  (bind _returnvalue (`self.GetInstigatorController` OtherActor))
  ;[1 1 1] Load into different level
  (if (`Controller.IsLocalPlayerController` _returnvalue)
    (bind _asbp_blockrun_controller (cast `/Game/_USER/Moz/Blueprints/BP_BlockrunController` _returnvalue))
    (set `/Game/_USER/Moz/Blueprints/BP_BlockrunController.ReturnZoneLoc` (`SceneComponent.K2_GetComponentToWorld` (`self.PlayerTeleportOut`)) _asbp_blockrun_controller)
    (if (`self.GM_NeedsTimer`)
      (bind _returnvalue_2 (`|CreateWidget` "/Game/Multiplayer/Widgets/WB_Loading.WB_Loading_C"))
      (`UserWidget.AddToViewport` _returnvalue_2 0))
    (`GameplayStatics.LoadStreamLevelBySoftObjectPtr` (`self.LevelToLoad`) true)
    (`/Game/_USER/Moz/Blueprints/BP_BlockrunController.Server_SetSpawnTransform` _asbp_blockrun_controller (`SceneComponent.K2_GetComponentToWorld` (`self.PlayerTeleport`)))
    (`/Game/_USER/Moz/Blueprints/BP_BlockrunController.Server_SpawnToLocation` _asbp_blockrun_controller (`self.GM_NeedsTimer`))
    (`KismetSystemLibrary.Delay` 0.5)
    (`/Engine/EditorBlueprintResources/StandardMacros.IsValid` _returnvalue_2
      (:`Is Valid`
        (`Widget.RemoveFromParent` _returnvalue_2)))))

(fn `UserConstructionScript`)