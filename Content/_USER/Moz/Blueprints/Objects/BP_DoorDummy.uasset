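; BP_DoorDummy is a door actor that streams in another level and teleports the player to it.
; Its entry box registers the door on the player's BP_BlockrunController, on authority only and while the door is closed.
; Its loader box stores a return transform, starts a non-blocking level load, and has the controller spawn the player at the teleport point.
; An optional loading widget, shown when GMNeedsTimer is set, is removed after a fixed delay.
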(event `self.COLL_EntryBox.OnComponentBeginOverlap`
  (params (OverlappedComponent :type "PrimitiveComponent Object Reference") (OtherActor :type "Actor Object Reference") (OtherComp :type "PrimitiveComponent Object Reference") (OtherBodyIndex :type Integer) (bFromSweep :type Boolean) (SweepResult :type "HitResult Structure (by ref)"))
  (`/Engine/EditorBlueprintResources/ActorMacros.Switch Has Authority`
    (:`Authority`
      (if (not (`self.IsDoorOpen`))
        (bind _asbp_blockrun_controller (cast `/Game/_USER/Moz/Blueprints/BP_BlockrunController` (`self.GetInstigatorController` OtherActor)))
        (set `/Game/_USER/Moz/Blueprints/BP_BlockrunController.CurrentDummyDoorRef` self _asbp_blockrun_controller)))))

(event `self.COLL_EntryBox.OnComponentEndOverlap`
  (params (OverlappedComponent :type "PrimitiveComponent Object Reference") (OtherActor :type "Actor Object Reference") (OtherComp :type "PrimitiveComponent Object Reference") (OtherBodyIndex :type Integer)))

(event `self.COLL_LevelLoader.OnComponentBeginOverlap`
  (params (OverlappedComponent :type "PrimitiveComponent Object Reference") (OtherActor :type "Actor Object Reference") (OtherComp :type "PrimitiveComponent Object Reference") (OtherBodyIndex :type Integer) (bFromSweep :type Boolean) (SweepResult :type "HitResult Structure (by ref)"))
  ;[1 1 1] Load into different level
  (bind _asbp_blockrun_controller (cast `/Game/_USER/Moz/Blueprints/BP_BlockrunController` (`self.GetInstigatorController` OtherActor)))
  (set `/Game/_USER/Moz/Blueprints/BP_BlockrunController.ReturnZoneLoc` (`SceneComponent.K2_GetComponentToWorld` (`self.PlayerTeleportOut`)) _asbp_blockrun_controller)
  (if (`self.GM_NeedsTimer`)
    (bind _returnvalue (`|CreateWidget` "/Game/Multiplayer/Widgets/WB_Loading.WB_Loading_C"))
    (`UserWidget.AddToViewport` _returnvalue 0))
  (`GameplayStatics.LoadStreamLevelBySoftObjectPtr` (`self.LevelToLoad`) true)
  (`/Game/_USER/Moz/Blueprints/BP_BlockrunController.Server_SetSpawnTransform` _asbp_blockrun_controller (`SceneComponent.K2_GetComponentToWorld` (`self.PlayerTeleport`)))
  (`/Game/_USER/Moz/Blueprints/BP_BlockrunController.Server_SpawnToLocation` _asbp_blockrun_controller (`self.GM_NeedsTimer`))
  (`KismetSystemLibrary.Delay` 0.5)
  (`/Engine/EditorBlueprintResources/StandardMacros.IsValid` _returnvalue
    (:`Is Valid`
      (`Widget.RemoveFromParent` _returnvalue))))

(fn `UserConstructionScript`)